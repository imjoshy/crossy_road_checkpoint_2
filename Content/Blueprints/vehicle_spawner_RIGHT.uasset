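; Vehicle spawner actor, named for the right side, that periodically spawns random traffic at its location.
; It uses a randomized tick interval as a spawn timer, choosing among police car, car and two truck types on each tick.
; A random multiplier picked at BeginPlay is passed to every vehicle, negated for Truck_1.
; Each tick also destroys the spawner once the player is over 500 units ahead of it in X.
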(event EventBeginPlay
  (Actor|Tick|SetActorTickInterval (Utilities|Select :Index (Math|Random|RandomIntegerinRange 0 2) :Option%200 1.0 :Option%201 2.0 :Option%202 3.0))
  (Variables|Default|Setmult (Utilities|Select :Index (Math|Random|RandomIntegerinRange 0 3) :Option%200 2 :Option%201 3 :Option%202 4 :Option%203 5)))

(event EventTick
  (params (DeltaSeconds :type Float%20%28single-precision%29))
  (bind _returnvalue (Transformation|GetActorLocation))
  (bind _returnvalue_2 (Transformation|GetActorLocation))
  (bind _returnvalue_3 (Transformation|GetActorLocation))
  (bind _returnvalue_4 (Transformation|GetActorLocation))
  (Actor|Tick|SetActorTickInterval (Utilities|Select :Index (Math|Random|RandomIntegerinRange 0 1) :Option%200 2.0 :Option%201 3.0))
  (Utilities|FlowControl|Sequence
    (:then_0
      (if (== (Math|Random|RandomIntegerinRange 0 1) 0)
        ;[1 1 1] spawn a car
        (if (== (Math|Random|RandomIntegerinRange 0 1) 0)
          ;;[1 1 1] spawn police car
          (bind _returnvalue_5 (Game|SpawnActorfromClass "/Game/Blueprints/police_car.police_car_C" (Math|Transform|MakeTransform (Math|Vector|MakeVector (+ (.x _returnvalue_3) 5e+01) (.y _returnvalue_3) -2e+01) "0,270.000000,90.000000" "25.000000,25.000000,25.000000") "Undefined" 0 0))
          (Variables|/Game/Blueprints/police_car.police_car_C|Setmultiplier _returnvalue_5 (Math|Conversions|ToFloat(Integer) (Variables|Default|Getmult)))
          (else
            ;;[1 1 1] spawn regular car
            (bind _returnvalue_6 (Game|SpawnActorfromClass "/Game/Blueprints/car.car_C" (Math|Transform|MakeTransform (Math|Vector|MakeVector (+ (.x _returnvalue_4) 5e+01) (.y _returnvalue_4) -2e+01) "0,270.000000,90.000000" "25.000000,25.000000,25.000000") "Undefined" 0 0))
            (Variables|/Game/Blueprints/car.car_C|Setmultiplier _returnvalue_6 (Math|Conversions|ToFloat(Integer) (Variables|Default|Getmult)))))
        (else
          ;[1 1 1] spawn a car
          (if (== (Math|Random|RandomIntegerinRange 0 1) 0)
            ;;[1 1 1] spawn police car
            (bind _returnvalue_7 (Game|SpawnActorfromClass "/Game/Blueprints/truck_1.truck_1_C" (Math|Transform|MakeTransform (Math|Vector|MakeVector (+ (.x _returnvalue) 0.0) (.y _returnvalue) -2e+01) "0,90.000000,90.000000" "25.000000,25.000000,25.000000") "Undefined" 0 0))
            (Variables|/Game/Blueprints/truck_1.truck_1_C|Setmultiplier _returnvalue_7 (Math|Conversions|ToFloat(Integer) (* (Variables|Default|Getmult) -1)))
            (else
              ;;[1 1 1] spawn regular car
              (bind _returnvalue_8 (Game|SpawnActorfromClass "/Game/Blueprints/truck_2.truck_2_C" (Math|Transform|MakeTransform (Math|Vector|MakeVector (+ (.x _returnvalue_2) 0.0) (.y _returnvalue_2) -2e+01) "0,90.000000,90.000000" "25.000000,25.000000,25.000000") "Undefined" 0 0))
              (Variables|/Game/Blueprints/truck_2.truck_2_C|Setmultiplier _returnvalue_8 (Math|Conversions|ToFloat(Integer) (Variables|Default|Getmult))))))))
    (:then_1
      (if (and (< (.x (Transformation|GetActorLocation)) (.x (Transformation|GetActorLocation (Game|GetPlayerCharacter 0)))) (> (- (Math|Float|Absolute(Float) (.x (Transformation|GetActorLocation (Game|GetPlayerCharacter 0)))) (Math|Float|Absolute(Float) (.x (Transformation|GetActorLocation)))) 5e+02))
        (Actor|DestroyActor)))))

(fn ConstructionScript)