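; Road spawner that builds a lane-crossing level along X, calling SpawnRoad three times on BeginPlay.
; Each call lays two road segments at an advancing X cursor, each with side barriers and two vehicle spawners randomly placed left or right.
; The second segment receives a reference back to this spawner.
; SpawnInitialRoad is not called here, and a grass-plus-road variant sits disconnected, marked for final submission.
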(event EventBeginPlay
  (CallFunction|SpawnRoad)
  (CallFunction|SpawnRoad)
  (CallFunction|SpawnRoad))

(event Collision|EventActorBeginOverlap
  (params (OtherActor :type Actor%20Object%20Reference)))

(event EventTick
  (params (DeltaSeconds :type Float%20%28single-precision%29)))

(fn ConstructionScript)

(fn SpawnInitialRoad
  (Game|SpawnActorfromClass "/Game/Blueprints/BP_grass.BP_grass_C" (Math|Transform|MakeTransform (Math|Vector|MakeVector (Variables|Default|Getspawn_loc_x) -5.9e+02 2e+01) "0, 0, 0" "1,1,1") "Undefined" 0 0) ; Spawn grass lane
  (bind _output_get (Variables|Default|Setspawn_loc_x (+ (Variables|Default|Getspawn_loc_x) 1.6e+02)))
  (Game|SpawnActorfromClass "/Game/Blueprints/BP_road.BP_road_C" (Math|Transform|MakeTransform (Math|Vector|MakeVector _output_get -5.9e+02 2e+01) "0, 0, 0" "1,1,1") "Undefined" 0 0) ; Spawn road lane
  (Utilities|FlowControl|Sequence ; Vehicle spawners on road lane
    (:then_0
      ;[1 1 1] First lane -- road spawn loc - 75
      (Variables|Default|Setvehicle_spawn_loc_x (- (Variables|Default|Getspawn_loc_x) 75.0))
      (CallFunction|SpawnVehicle))
    (:then_1
      ;[1 1 1] Second lane -- 70 ahead of first lane
      (Variables|Default|Setvehicle_spawn_loc_x (+ (Variables|Default|Getvehicle_spawn_loc_x) 7e+01))
      (CallFunction|SpawnVehicle)
      (Variables|Default|Setspawn_loc_x (+ (Variables|Default|Getspawn_loc_x) 1.6e+02)))))

(fn SpawnRoad
  ;[1 1 1] Roads only
  (Game|SpawnActorfromClass "/Game/Blueprints/BP_road.BP_road_C" (Math|Transform|MakeTransform (Math|Vector|MakeVector (Variables|Default|Getspawn_loc_x) -5.9e+02 (Variables|Default|Getroad_z)) "0, 0, 0" "1,1,1") "Undefined" 0 0)
  (CallFunction|SpawnBarriers)
  (Utilities|FlowControl|Sequence ; Vehicle spawners on road lane
    (:then_0
      ;;[1 1 1] First lane -- road spawn loc - 75
      (Variables|Default|Setvehicle_spawn_loc_x (- (Variables|Default|Getspawn_loc_x) 75.0))
      (CallFunction|SpawnVehicle))
    (:then_1
      ;;[1 1 1] Second lane -- 70 ahead of first lane
      (Variables|Default|Setvehicle_spawn_loc_x (+ (Variables|Default|Getvehicle_spawn_loc_x) 7e+01))
      (CallFunction|SpawnVehicle)
      (bind _output_get (Variables|Default|Setspawn_loc_x (+ (Variables|Default|Getspawn_loc_x) 1.6e+02)))
      (bind _returnvalue (Game|SpawnActorfromClass "/Game/Blueprints/BP_road.BP_road_C" (Math|Transform|MakeTransform (Math|Vector|MakeVector _output_get -5.9e+02 (Variables|Default|Getroad_z)) "0, 0, 0" "1,1,1") "Undefined" 0 0))
      (Variables|/Game/Blueprints/BP_road.BP_road_C|Setroad_spawner_ref _returnvalue self)
      (CallFunction|SpawnBarriers)
      (Utilities|FlowControl|Sequence ; Vehicle spawners on road lane
        (:then_0
          (Variables|Default|Setvehicle_spawn_loc_x (- (Variables|Default|Getspawn_loc_x) 75.0))
          (CallFunction|SpawnVehicle))
        (:then_1
          ;;[1 1 1] Second lane -- 70 ahead of first lane
          (Variables|Default|Setvehicle_spawn_loc_x (+ (Variables|Default|Getvehicle_spawn_loc_x) 7e+01))
          (CallFunction|SpawnVehicle)
          (Variables|Default|Setspawn_loc_x (+ (Variables|Default|Getspawn_loc_x) 1.6e+02)))))))

(fn SpawnVehicle
  (if (== (Math|Random|RandomIntegerinRange 0 1) 0)
    (CallFunction|SpawnVehicleLeft)
    (else
      (CallFunction|SpawnVehicleRight))))

(fn SpawnVehicleLeft
  (Game|SpawnActorfromClass "/Game/Blueprints/vehicle_spawner_LEFT.vehicle_spawner_LEFT_C" (Math|Transform|MakeTransform (Math|Vector|MakeVector (Variables|Default|Getvehicle_spawn_loc_x) -7e+02 0.0) "0, 0, 0" "1,1,1") "Undefined" 0 0))

(fn SpawnVehicleRight
  (Game|SpawnActorfromClass "/Game/Blueprints/vehicle_spawner_RIGHT.vehicle_spawner_RIGHT_C" (Math|Transform|MakeTransform (Math|Vector|MakeVector (Variables|Default|Getvehicle_spawn_loc_x) 7e+03 0.0) "0, 0, 0" "1,1,1") "Undefined" 0 0))

(fn SpawnBarriers
  ;[1 1 1] left barrier -- limit movement to the left
  (Game|SpawnActorfromClass "/Game/Blueprints/barrier.barrier_C" (Math|Transform|MakeTransform (Math|Vector|MakeVector (Variables|Default|Getspawn_loc_x) (Variables|Default|Getleft_most) 2e+01) "0, 0, 0" "1,1,1") "Undefined" 0 0)
  ;[1 1 1] right barrier -- limit movement to the right
  (Game|SpawnActorfromClass "/Game/Blueprints/barrier.barrier_C" (Math|Transform|MakeTransform (Math|Vector|MakeVector (Variables|Default|Getspawn_loc_x) (Variables|Default|Getright_most) 2e+01) "0, 0, 0" "1,1,1") "Undefined" 0 0))